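; BP_ky_fireBall is a fireball projectile that destroys what it hits, except BP_ThirdPersonCharacter actors.
; It spawns a tinted shockwave, then Tick moves it along local X using timeline-scaled speed plus a player max-speed term not scaled by delta time.
; A delay loop started from the timeline update fades it out when Duration expires.
; Overlaps not tagged ky_shot spawn hit effects, play explosion audio and destroy the fireball.
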(event EventBeginPlay
  (bind _defaultsceneroot (Variables|Default|GetDefaultSceneRoot))
  ;[1 1 1] spawn shot shockwave
  (bind _returnvalue (Effects|SpawnEmitteratLocation "/Game/GameContent/Effects/Particles/P_ky_shotShockwave.P_ky_shotShockwave" (Transformation|GetWorldLocation _defaultsceneroot) (Transformation|GetWorldRotation _defaultsceneroot)))
  (Effects|Components|ParticleSystem|SetVectorParameter _returnvalue "color" (Math|Conversions|ToVector(LinearColor) (Variables|Default|Getcolor)))
  ;[1 1 1] effect move correct
  (bind _valuecorrect (Timeline|Timeline_0 Play)
    (:Update
      (Variables|Default|SetspeedCorrect _valuecorrect)
      ;[1 1 1] duration control
      (Utilities|FlowControl|Delay 0.1 :!label _label)
      (if (< (Variables|Default|Getduration) 0.0)
        ;[1 1 1] fx deactivate
        (Collision|SetCollisionEnabled (Variables|Default|GetBox) "NoCollision")
        (Components|Activation|Deactivate (Variables|Default|GetFX1))
        (Utilities|FlowControl|Delay 1.0)
        ;[1 1 1] effect destroy
        (Actor|DestroyActor)
        (else
          (goto _label))))))

(event Collision|EventActorBeginOverlap
  (params (OtherActor :type Actor%20Object%20Reference))
  ;[1 1 1] spawn collison fx
  (if (Utilities|IsValid OtherActor)
    (if (Utilities|Name|NotEqual(Name) (Utilities|Array|Get(acopy) (Variables|/Script/Engine.Actor|GetTags OtherActor)) "ky_shot")
      (Effects|SpawnEmitteratLocation (Variables|Default|GethitFx) (Transformation|GetWorldLocation (Variables|Default|GetBox)))
      ;[1 1 1] fx destroy
      (Actor|DestroyActor)
      (Audio|PlaySound2D "/Game/GameContent/Sound/Explosion_Cue.Explosion_Cue" 1.0 1.0 0.0 0 0)
      (Utilities|Casting|CastToBP_ThirdPersonCharacter OtherActor ; Cant destroy character actor
        (:CastFailed
          (Actor|DestroyActor OtherActor))))))

(event EventTick
  (params (DeltaSeconds :type Float%20%28single-precision%29))
  ;[1 1 1] duration increment for control
  (Variables|Default|Setduration (- (Variables|Default|Getduration) DeltaSeconds))
  (bind _asbp_third_person_character (Utilities|Casting|CastToBP_ThirdPersonCharacter (Game|GetPlayerCharacter 0)))
  ;[1 1 1] move control
  (Transformation|AddActorLocalOffset (Math|Vector|MakeVector (+ (* (Variables|Default|Getspeed) (Variables|Default|GetspeedCorrect) (Utilities|Time|GetWorldDeltaSeconds)) (/ (Class|MovementComponent|GetMaxSpeed (Variables|/Script/Engine.Character|GetCharacterMovement _asbp_third_person_character)) 1e+01)) 0.0 0.0) false false))

(fn ConstructionScript)