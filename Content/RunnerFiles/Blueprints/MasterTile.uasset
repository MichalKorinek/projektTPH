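; MasterTile is an endless-runner track tile that spawns random obstacles across three lanes on BeginPlay.
; When the player exits its box, it asks the game mode for another tile, adds multiplier-scaled score and slightly raises walk speed within a clamp.
; After a short delay it destroys itself, its side blocks and tracked obstacles.
; Lane 0 alone can draw from a storm-inclusive class list, with a storm check that skips the other lanes.
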(event OnComponentEndOverlap(Box)
  (params (OverlappedComponent :type Primitive%20Component%20Object%20Reference) (OtherActor :type Actor%20Object%20Reference) (OtherComp :type Primitive%20Component%20Object%20Reference) (OtherBodyIndex :type Integer))
  (Utilities|Casting|CastToBP_ThirdPersonCharacter OtherActor)
  (bind _asbp_third_person_game_mode (Utilities|Casting|CastToBP_ThirdPersonGameMode (Game|GetGameMode)))
  (Default|SpawnTile _asbp_third_person_game_mode)
  (bind _asbp_third_person_game_mode_2 (Utilities|Casting|CastToBP_ThirdPersonGameMode (Game|GetGameMode)))
  (Variables|/Game/ThirdPerson/Blueprints/BP_ThirdPersonGameMode.BP_ThirdPersonGameMode_C|SetCurrentScore _asbp_third_person_game_mode_2 (+ (Variables|/Game/ThirdPerson/Blueprints/BP_ThirdPersonGameMode.BP_ThirdPersonGameMode_C|GetCurrentScore _asbp_third_person_game_mode_2) (* (Variables|/Game/ThirdPerson/Blueprints/BP_ThirdPersonGameMode.BP_ThirdPersonGameMode_C|GetMultiplier _asbp_third_person_game_mode_2) 1)))
  (bind _asbp_third_person_character (Utilities|Casting|CastToBP_ThirdPersonCharacter (Game|GetPlayerCharacter 0)))
  (Variables|/Script/Engine.CharacterMovementComponent|SetMaxWalkSpeed (Variables|/Script/Engine.Character|GetCharacterMovement _asbp_third_person_character) (Math|Float|Clamp(Float) (* (Variables|/Script/Engine.CharacterMovementComponent|GetMaxWalkSpeed (Variables|/Script/Engine.Character|GetCharacterMovement _asbp_third_person_character)) 1.01) 6e+02 1.6e+03))
  (Utilities|FlowControl|Delay 0.5)
  (Actor|DestroyActor)
  (for _array_element (Variables|Default|GetSideBlocks)
    (Actor|DestroyActor _array_element))
  (for _array_element_2 (Variables|Default|GetObstacles)
    (Utilities|IsValid _array_element_2
      (:Is%20Valid
        (Actor|DestroyActor _array_element_2)))))

(event EventBeginPlay
  (CallFunction|SpawnObstacles))

(fn ConstructionScript)

(fn SpawnObstacles
  ;[1 1 1] Lane0
  (switch int (Math|Random|RandomIntegerinRange 0 1)
    (:0
      ;[1 1 1] Lane 1
      (switch int (Math|Random|RandomIntegerinRange 0 1) :!label _label
        (:0
          _)
        (:1
          (bind _returnvalue (Game|SpawnActorfromClass (Utilities|Array|Get(acopy) (Variables|Default|GetObstaclesClasses) (Math|Random|RandomIntegerinRange 0 1)) (Math|Transform|MakeTransform (Transformation|GetWorldLocation (Variables|Default|GetLane1)) "0, 0, 0" "1.000000,1.000000,1.000000") "Undefined" 0 0))
          (Utilities|Array|Add (Variables|Default|GetObstacles) _returnvalue)))
      ;[1 1 1] Lane2
      (switch int (Math|Random|RandomIntegerinRange 0 1)
        (:1
          (bind _returnvalue_2 (Game|SpawnActorfromClass (Utilities|Array|Get(acopy) (Variables|Default|GetObstaclesClasses) (Math|Random|RandomIntegerinRange 0 1)) (Math|Transform|MakeTransform (Transformation|GetWorldLocation (Variables|Default|GetLane2)) "0, 0, 0" "1.000000,1.000000,1.000000") "Undefined" 0 0))
          (Utilities|Array|Add (Variables|Default|GetObstacles) _returnvalue_2))))
    (:1
      (bind _returnvalue_3 (Game|SpawnActorfromClass (Utilities|Array|Get(acopy) (Variables|Default|GetObstacleClassesWithStorm) (Math|Random|RandomIntegerinRange 0 2)) (Math|Transform|MakeTransform (Transformation|GetWorldLocation (Variables|Default|GetLane0)) "0, 0, 0" "1.000000,1.000000,1.000000") "Undefined" 0 0))
      (if (== _returnvalue_3 "/Game/FXVarietyPack/Blueprints/BP_ky_storm.BP_ky_storm")
        (Utilities|Array|Add (Variables|Default|GetObstacles) 0)
        (else
          (goto _label))))))